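; Gameplay Ability for a melee combo attack, playing AM_Melee_Combo on the avatar Character from its first section.
; Each ComboWindow.Start gameplay event checks ComboBuffer to either jump to the next montage section, up to three, or end the ability.
; The buffer is set only after that check, so as wired the first window event ends the ability.
; JumpAttack is empty, and older montage, switch and fall-attack chains are disconnected.
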(event Custom|TryContinueCombo
  ;[0.15 0.15 0.15 0.5] Try Continue Combo
  (if (Variables|Default|GetComboBuffer)
    (if (< (Variables|Default|GetComboIndex) 3)
      (bind _result (Math|Integer|IncrementInt (Variables|Default|GetComboIndex))
        (:%20%20
          (Variables|Default|SetComboBuffer false)
          (Ability|Animation|MontageJumptoSection (Utilities|Array|Get(acopy) (Variables|Default|GetStart%20Sections) _result))
          (CallFunction|WaitforCombo)))
      (else
        (Ability|EndAbility)))
    (else
      (Ability|EndAbility))))

(event Custom|ComboStart
  ;[0.15 0.15 0.15 0.5] Combo Start
  (Variables|Default|SetComboIndex 1)
  (Variables|Default|SetComboBuffer false)
  (Animation|Montage|PlayMontage (Variables|/Script/Engine.Character|GetMesh (stale Ability|EventActivateAbility _as캐릭터)) "/Game/Variant_Combat/Anims/AM_Melee_Combo.AM_Melee_Combo" 1.0 0.0 (Utilities|Array|Get(acopy) (Variables|Default|GetStart%20Sections) (Variables|Default|GetComboIndex))
    (:then
      (CallFunction|WaitforCombo))))

(event Custom|WaitForCombo
  ;[0.15 0.15 0.15 0.5] Wait For Combo
  (Ability|Tasks|WaitGameplayEvent "(TagName=\"Event.Character.ComboWindow.Start\")" 0
    (:EventReceived
      (CallFunction|TryContinueCombo)
      (Variables|Default|SetComboBuffer true))))

(event Custom|JumpAttack)

(event Ability|EventOnEndAbility
  (params (bWasCancelled :type Boolean))
  ;[0.15 0.15 0.15 0.5] 어빌리티 종료
  (Utilities|Casting|CastToCharacter (Ability|GetAvatarActorfromActorInfo))
  (Variables|Default|SetComboIndex 0)
  (Variables|Default|SetComboBuffer false))

(event Ability|EventActivateAbility
  (bind _as캐릭터 (Utilities|Casting|CastToCharacter (Ability|GetAvatarActorfromActorInfo))
    (:then
      (CallFunction|ComboStart))
    (:CastFailed
      (Ability|EndAbility))))