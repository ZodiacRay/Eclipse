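; Gameplay ability that checks whether a melee attack hits an actor.
; It reads two bone names from the triggering event's UBoneNameData object, then runs an instant WaitTargetData with TA_SphereTrace, which receives the bone data on spawn through C++, per the author's note.
; On a hit it prints the first actor's name and applies GE_AttackHit to the target data.
; The ability ends on hit, miss or cancel.
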(event Ability|EventActivateAbility
  ;[0.15 0.15 0.15 0.5] 때리는 본 구하기
  (bind _asbp_ubone_name_data (Utilities|Casting|CastToBP_UBoneNameData (.OptionalObject (Utilities|Struct|BreakGameplayEventData (Variables|Default|GetCurrentEventData)))))
  (Variables|Default|SetBoneNameA (Variables|/Game/GAS/BP_UBoneNameData.BP_UBoneNameData_C|GetBoneNameA _asbp_ubone_name_data))
  (Variables|Default|SetBoneNameB (Variables|/Game/GAS/BP_UBoneNameData.BP_UBoneNameData_C|GetBoneNameB _asbp_ubone_name_data))
  ;[0.15 0.15 0.15 0.5] TA_SphereTrace 생성시 BoneData 넘어감. (c++로 구현)
  (bind _data (|WaitTargetData :TaskInstanceName "HitCheckTask" :ConfirmationType "Instant" :Class "/Game/GAS/GA/Attack/TA_SphereTrace.TA_SphereTrace_C" :ReticleClass 0)
    (:then
      (if (Ability|TargetData|TargetDataHasActor _data)
        (Development|PrintString (Utilities|String|Append (Utilities|GetDisplayName (Utilities|Array|Get(acopy) (Ability|TargetData|GetActorsfromTargetData _data))) "got hit!"))
        (GameplayEffects|ApplyGameplayEffectToTarget _data "/Game/GAS/GE/Character/GE_AttackHit.GE_AttackHit_C" 1 1)
        (Ability|EndAbility)
        (else
          (Ability|EndAbility))))
    (:Cancelled
      (Ability|EndAbility))))

(event Ability|EventOnEndAbility
  (params (bWasCancelled :type Boolean)))