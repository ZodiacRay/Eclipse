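; GA_Death is a Gameplay Ability that handles a character's death.
; On activation it plays the front death montage and disables the avatar character's movement.
; When the montage completes, is interrupted or is cancelled, it turns off capsule collision, ragdolls the mesh, clears its overlay material, sets a short lifespan and ends the ability.
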(event Ability|EventActivateAbility
  (|PlayMontageandWaitProxy "Death Task" "/Game/03_Animations/AnimationAsset/Montage/Death/AM_Death_front.AM_Death_front" 1.0 "None" true 1.0 0.0 false
    (:then
      (bind _as캐릭터 (Utilities|Casting|CastToCharacter (Ability|GetAvatarActorfromActorInfo)))
      (Pawn|Components|CharacterMovement|SetMovementMode (Variables|/Script/Engine.Character|GetCharacterMovement _as캐릭터) "MOVE_None" 0))
    (:OnCompleted
      (Collision|SetCollisionEnabled (Variables|/Script/Engine.Character|GetCapsuleComponent _as캐릭터) "NoCollision" :!label _label)
      (Physics|SetSimulatePhysics (Variables|/Script/Engine.Character|GetMesh _as캐릭터) true)
      (Actor|SetLifeSpan _as캐릭터 3.0)
      (Rendering|Material|SetOverlayMaterial (Variables|/Script/Engine.Character|GetMesh _as캐릭터) 0 :!class /Script/Engine.MeshComponent)
      (Ability|EndAbility))
    (:OnInterrupted
      (goto _label))
    (:OnCancelled
      (goto _label))))

(event Ability|EventOnEndAbility
  (params (bWasCancelled :type Boolean)))