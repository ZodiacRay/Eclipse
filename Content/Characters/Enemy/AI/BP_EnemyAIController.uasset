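; AI controller for an enemy that tracks the player through AI perception updates.
; On each update, it checks whether player character 0 is among the updated actors, without checking whether the stimulus was sensed or lost.
; If present, it stores the player, sets the found flag and records the distance from the controller's owner.
; Otherwise, it clears the flag and sets the distance to a negative sentinel.
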(event OnPerceptionUpdated(AIPerception)
  (params (UpdatedActors :type Array%20of%20Actor%20Object%20References))
  (bind _returnvalue (Game|GetPlayerCharacter 0))
  (if (Utilities|Array|ContainsItem UpdatedActors _returnvalue)
    (bind _output_get (Variables|Default|SetPlayerCharacter _returnvalue))
    (Variables|Default|SetIsPlayerFound true)
    (Variables|Default|SetEnemyDistance (Math|Vector|VectorLength (- (Transformation|GetActorLocation (Components|GetOwner)) (Transformation|GetActorLocation _output_get))))
    (else
      (Variables|Default|SetIsPlayerFound false)
      (Variables|Default|SetEnemyDistance -1.0))))

(fn ConstructionScript)