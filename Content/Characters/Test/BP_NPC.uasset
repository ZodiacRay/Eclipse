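; BP_NPC is a test NPC character that uses AI perception to detect the player.
; Each perception update sets SeenPlayer from the stimulus result and, on a successful sense, stores the sensed BP_ThirdPersonCharacter in PlayerRef.
; Disconnected experimental nodes would fit the capsule half-height to the mesh's head socket, reposition the mesh and print the computed value, but they never run.
; Tick and the construction script are empty.
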(event OnTargetPerceptionUpdated(AIPerception)
  (params (Actor :type Actor%20Object%20Reference) (Stimulus :type AI%20Stimulus%20Structure))
  (bind _output_get (Variables|Default|SetSeen_Player (.bsuccessfullysensed Stimulus)))
  (if _output_get
    (bind _asbp_third_person_character (Utilities|Casting|CastToBP_ThirdPersonCharacter Actor))
    (Variables|Default|SetPlayerRef _asbp_third_person_character)))

(event EventTick
  (params (DeltaSeconds :type Float%20%28single-precision%29)))

(fn ConstructionScript)