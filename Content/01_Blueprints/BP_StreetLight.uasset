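; Street light actor that switches the look of its lamp material on and off.
; The construction script creates a dynamic instance of M_streetLight on mesh slot 1 and sets its emissive intensity and light color.
; Every Tick, IsActive selects either M_Emissive or DefaultMaterial and reapplies it to that same slot, replacing the configured dynamic instance at runtime.
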(event EventBeginPlay)

(event Collision|EventActorBeginOverlap
  (params (OtherActor :type Actor%20Object%20Reference)))

(event EventTick
  (params (DeltaSeconds :type Float%20%28single-precision%29))
  (bind _staticmesh (Variables|Default|GetStaticMesh))
  (if (Variables|Default|GetisActive?)
    (bind _output_get (Variables|Default|SetEmissive "/Game/TokyoStylizedEnvironment/Materials/Emissive_Light/M_Emissive.M_Emissive"))
    (Rendering|Material|SetMaterial _staticmesh 1 _output_get)
    (else
      (bind _output_get_2 (Variables|Default|SetEmissive "/Engine/EngineMaterials/DefaultMaterial.DefaultMaterial"))
      (Rendering|Material|SetMaterial _staticmesh 1 _output_get_2))))

(fn ConstructionScript
  (bind _returnvalue (Rendering|Material|CreateDynamicMaterialInstance (Variables|Default|GetStaticMesh) 1 "/Game/02_Materials/M_streetLight.M_streetLight" "None" :!class /Script/Engine.PrimitiveComponent))
  (bind _output_get (Variables|Default|SetLightMaterial _returnvalue))
  (Rendering|Material|SetScalarParameterValue _output_get "Emissive" (Variables|Default|GetLightIntensity) :!class /Script/Engine.MaterialInstanceDynamic)
  (Rendering|Material|SetVectorParameterValue _output_get "LightColor" (Variables|Default|GetLightColor) :!class /Script/Engine.MaterialInstanceDynamic))