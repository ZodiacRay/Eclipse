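; BP_FakeGLLight is an environment actor that fakes lighting with a mesh and material.
; The construction script applies the chosen Shape to LightMesh and assigns a dynamic instance of MI_FakeGL driven by the Brightness and LightColor variables.
; BeginPlay creates and assigns the dynamic material again with the same parameters, without resetting the mesh.
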(event EventBeginPlay
  (Utilities|FlowControl|Sequence
    (:then_0
      (bind _returnvalue (Rendering|Material|CreateDynamicMaterialInstance "/Game/01_Blueprints/Enviroment/FakeGlLight/MI_FakeGL.MI_FakeGL" "None" "None" :!class /Script/Engine.KismetMaterialLibrary))
      (bind _output_get (Variables|Default|SetDy_Material _returnvalue))
      (Rendering|Material|SetScalarParameterValue _output_get "Brightness" (Variables|Default|GetBrightness) :!class /Script/Engine.MaterialInstanceDynamic)
      (Rendering|Material|SetVectorParameterValue (Variables|Default|GetDy_Material) "LightColor" (Variables|Default|GetLightColor) :!class /Script/Engine.MaterialInstanceDynamic)
      (Rendering|Material|SetMaterial (Variables|Default|GetLightMesh) 0 (Variables|Default|GetDy_Material)))))

(fn ConstructionScript
  (Utilities|FlowControl|Sequence
    (:then_0
      (Components|StaticMesh|SetStaticMesh (Variables|Default|GetLightMesh) (Variables|Default|GetShape))
      (bind _returnvalue (Rendering|Material|CreateDynamicMaterialInstance "/Game/01_Blueprints/Enviroment/FakeGlLight/MI_FakeGL.MI_FakeGL" "None" "None" :!class /Script/Engine.KismetMaterialLibrary))
      (bind _output_get (Variables|Default|SetDy_Material _returnvalue))
      (Rendering|Material|SetScalarParameterValue _output_get "Brightness" (Variables|Default|GetBrightness) :!class /Script/Engine.MaterialInstanceDynamic)
      (Rendering|Material|SetVectorParameterValue (Variables|Default|GetDy_Material) "LightColor" (Variables|Default|GetLightColor) :!class /Script/Engine.MaterialInstanceDynamic)
      (Rendering|Material|SetMaterial (Variables|Default|GetLightMesh) 0 (Variables|Default|GetDy_Material)))))