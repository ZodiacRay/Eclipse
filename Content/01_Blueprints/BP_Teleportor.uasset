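; Teleporter actor that glides any actor overlapping its Trigger over to a referenced TeleportActor.
; On overlap, it caches raised start and destination points, then a double-speed timeline lerps the actor's location between them without sweeping.
; A busy flag (NewVar) ignores further overlaps until shortly after the move finishes.
; The BeginPlay validity check does nothing, and an alternative Teleport call is left unconnected.
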(event OnComponentBeginOverlap(Trigger)
  (params (OverlappedComponent :type Primitive%20Component%20Object%20Reference) (OtherActor :type Actor%20Object%20Reference) (OtherComp :type Primitive%20Component%20Object%20Reference) (OtherBodyIndex :type Integer) (bFromSweep :type Boolean) (SweepResult :type Hit%20Result%20Structure%20%28by%20ref%29))
  (if (not (Variables|Default|GetNewVar))
    (bind _output_get (Variables|Default|SetOther%20Actor OtherActor))
    ;[0.15 0.15 0.15 0.5] 출발지점
    (Variables|Default|SetLocationA (+ (Transformation|GetActorLocation _output_get) "0.000000,0.000000,100.000000"))
    ;[0.15 0.15 0.15 0.5] 도착지점
    (Variables|Default|SetLocationB (+ (Transformation|GetActorLocation (Variables|Default|GetTeleportActor)) "0.000000,0.000000,100.000000"))
    (Variables|Default|SetNewVar true)
    (Components|Timeline|SetPlayRate (Variables|Default|GetTeleporting) 2.0)
    (bind _teleport (Timeline|Teleporting PlayFromStart)
      (:Update
        (Transformation|SetActorLocation (Variables|Default|GetOther%20Actor) (Math|Vector|Lerp(Vector) (Variables|Default|GetLocationA) (Variables|Default|GetLocationB) _teleport) false false))
      (:Finished
        (Utilities|FlowControl|Delay 1.0)
        (Variables|Default|SetNewVar false)))))

(event EventBeginPlay
  (Utilities|IsValid (Variables|Default|GetTeleportActor)))

(fn ConstructionScript)