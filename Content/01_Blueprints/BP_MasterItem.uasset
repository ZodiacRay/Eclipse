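; BP_MasterItem is an item actor, apparently a base for items, that shows an interaction hint when the player character is nearby.
; Sphere overlap, gated by CanInteract, creates a UI_Interact widget, plays its PopUp animation, applies an outline overlay material and sets CanPressE.
; Leaving reverses the animation, clears the outline and removes the widget after a short delay.
; CanReceiveTrace can replay or hide the hint while CanPressE is set.
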(event OnComponentBeginOverlap(Sphere)
  (params (OverlappedComponent :type Primitive%20Component%20Object%20Reference) (OtherActor :type Actor%20Object%20Reference) (OtherComp :type Primitive%20Component%20Object%20Reference) (OtherBodyIndex :type Integer) (bFromSweep :type Boolean) (SweepResult :type Hit%20Result%20Structure%20%28by%20ref%29))
  (bind _widget (Variables|Default|GetWidget))
  ;[0.15 0.15 0.15 0.5] 플레이어가 범위 내 들어온 경우
  (Utilities|Casting|CastToBP_ThirdPersonCharacter OtherActor)
  ;;[0.15 0.15 0.15 0.5] 상호작용 가능한 경우
  (if (Variables|Interaction|GetCanInteract)
    ;;[0.15 0.15 0.15 0.5] UI 생성
    (bind _returnvalue (UserInterface|CreateWidget "/Game/04_UI/BPUI/UI_Interact.UI_Interact_C"))
    (bind _output_get (Variables|상호작용|SetInteractionWidget _returnvalue))
    (UserInterface|SetWidget _widget _output_get)
    (Rendering|SetVisibility _widget true false)
    (bind _interactionwidget (Variables|상호작용|GetInteractionWidget)
      (:then
        ;;[0.15 0.15 0.15 0.5] UI 애니메이션 재생
        (if (not (Variables|상호작용|GetHintVisible))
          (Variables|상호작용|SetHintVisible true)
          (UserInterface|Animation|PlayAnimation _interactionwidget (Variables|/Game/04_UI/BPUI/UI_Interact.UI_Interact_C|GetPopUp _interactionwidget) 0.0 1 "Forward" 1.5 false)
          (Rendering|Material|SetOverlayMaterial (Variables|Default|GetStaticMesh) "/Game/04_UI/BPUI/M_Outline.M_Outline" :!class /Script/Engine.MeshComponent)
          (Variables|상호작용|SetCanPressE true)))
      (:else))))

(event OnComponentEndOverlap(Sphere)
  (params (OverlappedComponent :type Primitive%20Component%20Object%20Reference) (OtherActor :type Actor%20Object%20Reference) (OtherComp :type Primitive%20Component%20Object%20Reference) (OtherBodyIndex :type Integer))
  ;[0.15 0.15 0.15 0.5] 플레이어가 범위를 나간 경우
  (Utilities|Casting|CastToBP_ThirdPersonCharacter OtherActor)
  ;;[0.15 0.15 0.15 0.5] 상호작용 할 수 있는 경우
  (if (Variables|Interaction|GetCanInteract)
    (bind _interactionwidget (Variables|상호작용|GetInteractionWidget)
      (:then
        (if (Variables|상호작용|GetHintVisible)
          (UserInterface|Animation|PlayAnimation _interactionwidget (Variables|/Game/04_UI/BPUI/UI_Interact.UI_Interact_C|GetPopUp _interactionwidget) 0.0 1 "Reverse" 1.5 false)
          (Variables|상호작용|SetHintVisible false)
          (Variables|상호작용|SetCanPressE false)
          (Rendering|Material|SetOverlayMaterial (Variables|Default|GetStaticMesh) 0 :!class /Script/Engine.MeshComponent))
        (Utilities|FlowControl|Delay 0.15)
        (Widget|RemovefromParent (Variables|상호작용|GetInteractionWidget))
        (Variables|상호작용|SetInteractionWidget 0)
        (Rendering|SetVisibility (Variables|Default|GetWidget) false false))
      (:else))))

(event EventCanReceiveTrace
  (params (CanInteract :type Boolean))
  (if (Variables|상호작용|GetCanPressE)
    (if CanInteract
      (bind _interactionwidget (Variables|상호작용|GetInteractionWidget)
        (:then
          (if (Variables|상호작용|GetHintVisible)
            (UserInterface|Animation|PlayAnimation _interactionwidget (Variables|/Game/04_UI/BPUI/UI_Interact.UI_Interact_C|GetPopUp _interactionwidget) 0.0 1 "Forward" 1.5 false)
            (Variables|상호작용|SetHintVisible true)
            (Rendering|Material|SetOverlayMaterial (Variables|Default|GetStaticMesh) "/Game/04_UI/BPUI/M_Outline.M_Outline" :!class /Script/Engine.MeshComponent)
            (Variables|상호작용|SetCanPressE true)))
        (:else))
      (else
        (bind _interactionwidget_2 (Variables|상호작용|GetInteractionWidget)
          (:then
            (if (Variables|상호작용|GetHintVisible)
              (UserInterface|Animation|PlayAnimation _interactionwidget_2 (Variables|/Game/04_UI/BPUI/UI_Interact.UI_Interact_C|GetPopUp _interactionwidget_2) 0.0 1 "Reverse" 1.5 false)
              (Variables|상호작용|SetHintVisible false)
              (Rendering|Material|SetOverlayMaterial (Variables|Default|GetStaticMesh) 0 :!class /Script/Engine.MeshComponent)
              (Variables|상호작용|SetCanPressE false)))
          (:else))))))

(fn ConstructionScript)