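; GA_EquipWeapon is an event-triggered gameplay ability that equips or unequips the avatar's weapon.
; It commits, then switches on the first target tag in the event data.
; Bow and Sword tags pass their weapon Blueprint to the avatar's WeaponManagerComponent, while any other tag unequips.
; The ability ends immediately afterward, or directly if the component is missing.
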(event Ability|EventActivateAbility)

(event Ability|EventOnEndAbility
  (params (bWasCancelled :type Boolean)))

(event Ability|EventActivateAbilityFromEvent
  (params (EventData :type Gameplay%20Event%20Data%20Structure%20%28by%20ref%29))
  (bind _returnvalue (Ability|GetAvatarActorfromActorInfo))
  (bind _returnvalue_2 (Actor|GetComponentbyClass _returnvalue "/Game/01_Blueprints/03_Weapon/WeaponManagerComponent.WeaponManagerComponent_C"))
  (Ability|CommitAbility)
  (Utilities|IsValid _returnvalue_2
    (:Is%20Valid
      (Utilities|FlowControl|Sequence
        (:then_0
          (|SwitchGameplayTag (Utilities|Array|Get(acopy) (GameplayTags|BreakGameplayTagContainer (.TargetTags (Utilities|Struct|BreakGameplayEventData EventData))))
            (:Default
              (Default|UnequipWeapon _returnvalue_2))
            (:weapon.type.Bow
              (Default|EquipWeapon _returnvalue_2 "/Game/01_Blueprints/03_Weapon/BP_Weapon_Bow.BP_Weapon_Bow_C"))
            (:weapon.type.Sword
              (Default|EquipWeapon _returnvalue_2 "/Game/01_Blueprints/03_Weapon/BP_Weapon_Sword.BP_Weapon_Sword_C"))))
        (:then_1
          (Ability|EndAbility :!label _label))))
    (:Is%20Not%20Valid
      (goto _label))))