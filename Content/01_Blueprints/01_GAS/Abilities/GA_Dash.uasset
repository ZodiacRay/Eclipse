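; Gameplay ability that dashes the avatar pawn along its last movement input, or its forward vector when there is no input.
; It commits cost on activation, then applies a short constant root motion force that clamps exit velocity to the pawn's max speed.
; An active dash gameplay cue plays until the ability ends.
; Cooldown is committed only when the dash finishes, just before EndAbility.
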(event Ability|EventActivateAbility
  ;[0.15 0.15 0.15 0.5] 코스트는 어빌리티 실행전 처리
  (Ability|CommitAbilityCost false)
  ;[0.15 0.15 0.15 0.5] 벽을 뚫는 등의 충돌 처리 필요 x
  (Ability|Tasks|ApplyRootMotionConstantForce "None" (CallFunction|GetDashDirection) 2e+03 0.3 false 0 "ClampVelocity" "0, 0, 0" (CallFunction|GetMaxSpeed)
    (:then
      ;[0.15 0.15 0.15 0.5] Cue 호출
      (GameplayCue|AddGameplayCue :GameplayCueTag "(TagName=\"GameplayCue.Dash.Active\")"))
    (:OnFinish
      ;[0.15 0.15 0.15 0.5] 쿨타임은 어빌리티가 실행된 후 적용
      (Ability|CommitAbilityCooldown false)
      (Ability|EndAbility))))

(event Ability|EventOnEndAbility
  (params (bWasCancelled :type Boolean)))

(fn GetDashDirection
  (bind _returnvalue (Ability|GetAvatarActorfromActorInfo))
  (bind _aspawn (Utilities|Casting|CastToPawn _returnvalue))
  (if (Math|Vector|VectorIsZero (Class|Pawn|GetLastMovementInputVector _aspawn))
    ;[0.15 0.15 0.15 0.5] 캐릭터 앞 방향
    (return (Transformation|GetActorForwardVector _returnvalue))
    (else
      ;[0.15 0.15 0.15 0.5] 마지막 입력 방향
      (return (Class|Pawn|GetLastMovementInputVector _aspawn)))))

(fn GetMaxSpeed
  (bind _aspawn (Utilities|Casting|CastToPawn (Ability|GetAvatarActorfromActorInfo)))
  (return (Class|MovementComponent|GetMaxSpeed (Pawn|GetMovementComponent _aspawn))))