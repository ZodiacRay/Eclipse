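; BP_MasterItem_Child is an interactable item that swings its static mesh 90 degrees in yaw, toggling like a hinged door.
; BeginPlay caches the mesh's starting rotation.
; Interact, gated by CanPressE and CanInteract, flips Opened and plays or reverses TL_Rotate, which lerps yaw from that cached value.
; Timeline updates trigger a short Delay that re-enables both flags, acting as an input cooldown.
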(event EventBeginPlay
  (Variables|Default|SetStarting%20Roatation (Variables|/Script/Engine.SceneComponent|GetRelativeRotation (Variables|Default|GetStaticMesh))))

(event Collision|EventActorBeginOverlap
  (params (OtherActor :type Actor%20Object%20Reference)))

(event EventTick
  (params (DeltaSeconds :type Float%20%28single-precision%29)))

(event EventInteract
  (bind _starting_roatation (Variables|Default|GetStarting%20Roatation))
  (if (Variables|Default|GetCanPressE)
    (if (Variables|Default|GetCanInteract)
      (Variables|Default|SetCanInteract false)
      (if (Variables|Default|GetOpened)
        (Variables|Default|SetOpened false)
        (bind _새_트랙_0 (Timeline|TL_Rotate PlayFromStart)
          (:Update
            (Transformation|SetRelativeRotation (Variables|Default|GetStaticMesh) (Math|Rotator|MakeRotator (.roll _starting_roatation) (.pitch _starting_roatation) (Math|Float|Lerp (.yaw _starting_roatation) (- (.yaw _starting_roatation) 9e+01) _새_트랙_0)) false false)
            (Utilities|FlowControl|Delay 0.2)
            (Variables|Default|SetCanInteract true)
            (Variables|Default|SetCanPressE true)))
        (else
          (Variables|Default|SetOpened true)
          (Timeline|TL_Rotate Reverse))))))

(fn ConstructionScript
  (|CallParentFunction))